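; Template actor showing how to use an ASerial serial device, configured here with example ergometer settings.
; On BeginPlay it sets ID, version and name, creates the device, binds its data-received event and enables player input if creation succeeds.
; Releasing G sends a data request command, and received values print to screen.
; Unwired example nodes show thread pause, restart, frequency change and connection control.
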(event `self.ReceiveBeginPlay`
  (`self.InitializeDevice`)
  (bind _returnvalue (`ASerialComBPLibrary.CreateDevice` (`self.Device ID`) (`self.Device Version`) (`self.Name`)))
  (`/Engine/EditorBlueprintResources/StandardMacros.IsValid` _returnvalue
    (:`Is Valid`
      (set `self.Device` _returnvalue)
      (add `WiredDevice.OnRecieveDataEvent` (`self.Device`) (delegate `OnDataRecieve`))
      ;[1 1 1] Enable Inputが呼ばれだから下のキーボード入力が作動する
      (`self.EnableInput` (`GameplayStatics.GetPlayerController` 0)))))

(event `OnDataRecieve`
  (params (Value :type Integer))
  ;[1 1 1] データが貰ったの後処理
  (`KismetSystemLibrary.PrintString` (`KismetStringLibrary.Concat_StrStr` "貰ったデータ：" (`KismetStringLibrary.Conv_IntToString` Value)) true false))

(event `Key|G`
  (params (Key :type "Key Structure"))
  (:`Released`
    ;[1 1 1] データを要求する
    ; コマンドはエルゴメーターのデータ、実際どうなるかは電子科から貰った資料を見てください
    (`WiredDevice.RequestData` (`self.Device`) (`self.Cmd`))))

(fn `InitializeDevice`
  ;[1 1 1] これはエルゴメーターのデータ、実際どうなるかは電子科から貰った資料を見てください
  (set `self.Device ID` 3)
  (set `self.Device Version` 3)
  (set `self.Name` "TestName"))

(fn `UserConstructionScript`)