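; BP_Door2 is a sliding door actor that opens and closes in response to its SetActivationState event.
; It records its start location on BeginPlay, then plays a timeline when the condition is met and reverses it otherwise.
; The timeline's MoveDoorY track offsets the whole actor along its right vector from that start, without sweeping, and each state change prints a debug string.
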(event `self.ReceiveBeginPlay`
  (set `self.StartLocation` (`self.K2_GetActorLocation`)))

(event `StatefulActivatableInterface.SetActivationState`
  (params (bConditionMet :type Boolean) (Activator :type "Actor Object Reference"))
  (if bConditionMet
    (`KismetSystemLibrary.PrintString` "DoorOpen")
    (bind (_direction _movedoory) (`Timeline|タイムライン` :!label _label)
      (:`Update`
        (`self.K2_SetActorLocation` (+ (`self.StartLocation`) (* _movedoory (`self.GetActorRightVector`))))))
    (else
      (`KismetSystemLibrary.PrintString` "DoorClose")
      (goto _label :!via `Reverse`))))

(fn `UserConstructionScript`)